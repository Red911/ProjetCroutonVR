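; BP_Alarme is a spaceship alarm light that switches on when electrical power is cut and off when it starts.
; On BeginPlay it binds to the start and cut electricity dispatchers of a referenced battery slot.
; A power cut plays a timeline that drives the point light's intensity through a scaled curve, while power start stops the timeline and zeroes the intensity.
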(event Custom|TurnOff
  (Rendering|Components|Light|SetIntensity (Variables|Default|GetPointLight) 0.0)
  (bind _newtrack_0 (Timeline|Timeline Stop)
    (:Update
      (Rendering|Components|Light|SetIntensity (Variables|Default|GetPointLight) (* _newtrack_0 1e+03)))))

(event Custom|TurnON
  (bind _newtrack_0 (Timeline|Timeline PlayFromStart)
    (:Update
      (Rendering|Components|Light|SetIntensity (Variables|Default|GetPointLight) (* _newtrack_0 1e+03)))))

(event EventBeginPlay
  (bind _batterieslotref (Variables|Default|GetBatterieSlotRef))
  (EventDispatchers|BindEventtoEDStartElec _batterieslotref (delegate Custom|TurnOff))
  (EventDispatchers|BindEventtoEDCutElec _batterieslotref (delegate Custom|TurnON)))

(fn ConstructionScript)