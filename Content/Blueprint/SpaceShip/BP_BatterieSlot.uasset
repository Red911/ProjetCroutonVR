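; BP_BatterieSlot is a VR spaceship battery socket that switches electricity on and off.
; When a BP_Batterie enters the Box, it releases the grab, disables physics, clears the VRPawn's held-hand reference and snaps the overlapping component to BatteriePositionPoint.
; It then fires the StartElec event dispatcher; the battery leaving the Box fires CutElec, so listeners handle the actual power change.
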(event OnComponentBeginOverlap(Box)
  (params (OverlappedComponent :type Primitive%20Component%20Object%20Reference) (OtherActor :type Actor%20Object%20Reference) (OtherComp :type Primitive%20Component%20Object%20Reference) (OtherBodyIndex :type Integer) (bFromSweep :type Boolean) (SweepResult :type Hit%20Result%20Structure%20%28by%20ref%29))
  (bind _batteriepositionpoint (Variables|Default|GetBatteriePositionPoint))
  (bind _asbp_batterie (Utilities|Casting|CastToBP_Batterie OtherActor))
  (Default|TryRelease (Variables|/Game/Blueprint/SpaceShip/BP_Batterie.BP_Batterie_C|GetGrabComponent _asbp_batterie))
  (Physics|SetSimulatePhysics (Variables|/Game/Blueprint/SpaceShip/BP_Batterie.BP_Batterie_C|GetCube _asbp_batterie) false)
  (CallFunction|ClearObjectsHeldbyHands (Variables|/Game/Blueprint/SpaceShip/BP_Batterie.BP_Batterie_C|GetGrabComponent _asbp_batterie))
  (Transformation|SetWorldLocation OtherComp (Transformation|GetWorldLocation _batteriepositionpoint) false false)
  (Transformation|SetWorldRotation OtherComp (Transformation|GetWorldRotation _batteriepositionpoint) false false)
  (Default|CallEDStartElec)
  (Development|PrintString "Start Elec"))

(event OnComponentEndOverlap(Box)
  (params (OverlappedComponent :type Primitive%20Component%20Object%20Reference) (OtherActor :type Actor%20Object%20Reference) (OtherComp :type Primitive%20Component%20Object%20Reference) (OtherBodyIndex :type Integer))
  (Utilities|Casting|CastToBP_Batterie OtherActor)
  (Default|CallEDCutElec)
  (Development|PrintString "CUtElect"))

(fn ConstructionScript)

(fn ClearObjectsHeldbyHands
  (params (GrabComponent :type Grab%20Component%20Object%20Reference))
  (bind _asvrpawn (Utilities|Casting|CastToVRPawn (Game|Player|GetPlayerPawn 0)))
  (if (Utilities|Enum|Equal(Enum) (Default|GetHeldbyHand GrabComponent) "Left")
    (Variables|/Game/VRTemplate/Blueprints/VRPawn.VRPawn_C|SetHeldComponentLeft _asvrpawn 0)
    (else
      (Variables|/Game/VRTemplate/Blueprints/VRPawn.VRPawn_C|SetHeldComponentRight _asvrpawn 0))))