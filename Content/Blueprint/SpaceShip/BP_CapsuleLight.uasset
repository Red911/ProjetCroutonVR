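; BP_CapsuleLight is a spaceship capsule light that responds to power changes from a referenced battery slot.
; On BeginPlay it binds to the slot's start and cut electricity event dispatchers.
; Each event restarts its own timeline, whose track value is scaled by a fixed multiplier to drive the point light's intensity.
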(event Custom|StartElec
  (bind _newtrack_0 (Timeline|Timeline_0 PlayFromStart)
    (:Update
      (Rendering|Components|Light|SetIntensity (Variables|Default|GetPointLight) (* _newtrack_0 4e+02)))))

(event Custom|CutElec
  (bind _newtrack_0 (Timeline|Timeline PlayFromStart)
    (:Update
      (Rendering|Components|Light|SetIntensity (Variables|Default|GetPointLight) (* _newtrack_0 4e+02)))))

(event EventBeginPlay
  (bind _batterieslotref (Variables|Default|GetBatterieSlotRef))
  (EventDispatchers|BindEventtoEDStartElec _batterieslotref (delegate Custom|StartElec))
  (EventDispatchers|BindEventtoEDCutElec _batterieslotref (delegate Custom|CutElec)))

(fn ConstructionScript)