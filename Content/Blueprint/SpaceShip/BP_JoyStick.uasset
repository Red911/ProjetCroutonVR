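; VR grabbable spaceship joystick that steers a controlled object through BPI_Joystickable.
; On grab, a Cube attaches to the motion controller as a rotation proxy, then reattaches to the root on release.
; Each tick, its clamped roll/pitch delta from the grab tilts the Scene component and, while held, is sent normalized as movement or, for secondary sticks, rotation input.
; Battery slot events set IsElec, which never gates input here.
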(event OnGrabbed(GrabComponent)
  (bind _grabcomponent (Variables|Default|GetGrabComponent))
  (bind _cube (Variables|Default|GetCube))
  (if (Variables|/Game/VRTemplate/Blueprints/GrabComponent.GrabComponent_C|GetbIsHeld _grabcomponent)
    (bind _motioncontrollerref (Variables|/Game/VRTemplate/Blueprints/GrabComponent.GrabComponent_C|GetMotionControllerRef _grabcomponent)
      (:then
        (Variables|Default|SetNewVar_0 (Transformation|GetAttachParent _cube))
        (Transformation|AttachComponentToComponent _cube _motioncontrollerref "None" "KeepWorld" "KeepWorld" "KeepWorld" true)
        (Variables|Default|Settest (Transformation|GetWorldRotation (Variables|Default|GetCube))))
      (:else))))

(event OnDropped(GrabComponent)
  (bind _cube (Variables|Default|GetCube))
  (bind _grabcomponent (Variables|Default|GetGrabComponent))
  (bind _defaultsceneroot (Variables|Default|GetDefaultSceneRoot))
  (bind _returnvalue (Transformation|GetWorldRotation _defaultsceneroot))
  (if (not (Variables|/Game/VRTemplate/Blueprints/GrabComponent.GrabComponent_C|GetbIsHeld _grabcomponent))
    (Variables|/Game/VRTemplate/Blueprints/GrabComponent.GrabComponent_C|GetMotionControllerRef _grabcomponent
      (:then
        (Transformation|AttachComponentToComponent _cube (Variables|Default|GetDefaultSceneRoot) "None" "KeepWorld" "KeepWorld" "KeepWorld" true)
        (Transformation|SetRelativeRotation (Variables|Default|GetScene) _returnvalue false false)
        (Transformation|SetRelativeRotation _cube _returnvalue false false)
        (Transformation|SetRelativeLocation _cube (Variables|/Script/Engine.SceneComponent|GetRelativeLocation (Variables|Default|GetLevier)) false false))
      (:else))))

(event Custom|StartElec
  (Variables|Default|SetIsElec true))

(event Custom|CutElec
  (Variables|Default|SetIsElec false))

(event EventBeginPlay
  (bind _batterieslotref (Variables|Default|GetBatterieSlotRef))
  (EventDispatchers|BindEventtoEDStartElec _batterieslotref (delegate Custom|StartElec))
  (EventDispatchers|BindEventtoEDCutElec _batterieslotref (delegate Custom|CutElec)))

(event EventTick
  (params (DeltaSeconds :type Float%20%28single-precision%29))
  (bind _cube (Variables|Default|GetCube))
  (bind _test (Variables|Default|Gettest))
  (bind _scene (Variables|Default|GetScene))
  (bind _controlledojectref (Variables|Default|GetControlledOjectRef))
  (bind _returnvalue (Transformation|GetWorldRotation _cube))
  (bind _returnvalue_2 (Math|Rotator|Delta(Rotator) _test _returnvalue))
  (bind _returnvalue_3 (Math|Float|Clamp(Float) (.roll _returnvalue_2) -45.0 45.0))
  (bind _returnvalue_4 (Math|Float|Clamp(Float) (.pitch _returnvalue_2) -45.0 45.0))
  (bind _returnvalue_5 (Math|Float|Round _returnvalue_4))
  (bind _returnvalue_6 (Math|Float|Round _returnvalue_3))
  (bind _returnvalue_7 (Math|Conversions|ToFloat(Integer) _returnvalue_6))
  (bind _returnvalue_8 (Math|Conversions|ToFloat(Integer) _returnvalue_5))
  (bind _returnvalue_9 (Math|Vector2D|MakeVector2D _returnvalue_7 _returnvalue_8))
  (bind _returnvalue_10 (Math|Vector2D|Normalize2D _returnvalue_9))
  (bind _returnvalue_11 (Math|Conversions|ToVector(Vector2D) _returnvalue_10))
  (Transformation|SetRelativeRotation _scene (Math|Rotator|Lerp(Rotator) (Math|Rotator|MakeRotator _returnvalue_3 _returnvalue_4 0.0) (Transformation|GetWorldRotation _scene) 0.001) false false)
  (if (Utilities|DoesObjectImplementInterface _controlledojectref "/Game/Blueprint/Interface/BPI_Joystickable.BPI_Joystickable_C")
    (if (Variables|/Game/VRTemplate/Blueprints/GrabComponent.GrabComponent_C|GetbIsHeld (Variables|Default|GetGrabComponent))
      (if (Variables|Default|GetisSecondaryJoystick)
        (Class|BPIJoystickable|JoystickInputRot(Message) _controlledojectref _returnvalue_11)
        (else
          (Class|BPIJoystickable|JoystickInput(Message) _controlledojectref _returnvalue_11)))
      (else
        (Transformation|SetRelativeRotation (Variables|Default|GetScene) "0, 0, 0" false false)))))

(event EventGrab
  (params (MotionController :type Motion%20Controller%20Component%20Object%20Reference))
  (Variables|Default|SetMotion%20Controller MotionController))

(event EventRelease
  (params (MotionController :type Motion%20Controller%20Component%20Object%20Reference))
  (if (== MotionController (Variables|Default|GetMotion%20Controller))
    (Variables|Default|SetMotion%20Controller 0)))

(fn ConstructionScript)