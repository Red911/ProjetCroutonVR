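; BP_Levier is a spaceship lever that follows a motion controller while grabbed.
; Grab stores the controller, and Release clears it only when the same controller lets go.
; Each Tick converts the controller's position into the lever's space with a 90-degree offset, then adds the look-at pitch to the current pitch, clamped to a quarter turn with roll and yaw zeroed.
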(event EventGrab
  (params (MotionController :type Motion%20Controller%20Component%20Object%20Reference))
  (Variables|Default|SetMotion%20Controller MotionController))

(event EventRelease
  (params (MotionController :type Motion%20Controller%20Component%20Object%20Reference))
  (if (== MotionController (Variables|Default|GetMotion%20Controller))
    (Variables|Default|SetMotion%20Controller 0)))

(event EventTick
  (params (DeltaSeconds :type Float%20%28single-precision%29))
  (bind _levier (Variables|Default|GetLevier))
  (bind _returnvalue (Transformation|GetWorldTransform _levier))
  (bind _motion_controller (Variables|Default|GetMotion%20Controller)
    (:then
      (Transformation|SetRelativeRotation (Variables|Default|GetLevier) (Math|Rotator|MakeRotator 0.0 (Math|Float|Clamp(Float) (+ (.pitch (Variables|/Script/Engine.SceneComponent|GetRelativeRotation (Variables|Default|GetLevier))) (.pitch (Math|Rotator|FindLookatRotation (Math|Vector|MakeVector 0.0 0.0 0.0) (.location (Math|Transform|MakeRelativeTransform (Transformation|GetWorldTransform _motion_controller) (Math|Transform|MakeTransform (.location _returnvalue) (Math|Rotator|CombineRotators (.rotation _returnvalue) "90.000000,0.000000,0.000000") (.scale _returnvalue))))))) 0.0 9e+01) 0.0) false false))
    (:else)))

(fn ConstructionScript)