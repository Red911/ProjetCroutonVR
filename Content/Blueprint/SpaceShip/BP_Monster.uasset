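; BP_Monster is a monster that teleports around the spaceship and can trigger an oxygen leak.
; Tick moves it to a random ship waypoint, using a Delay and flag to wait TpTime between jumps.
; When close to the ship's Parent component with power on, it launches the leak once, as HaveAttacked never resets.
; BP_BatterieSlot's power cut and restore events toggle IsElecCut, which blocks the attack but not teleporting.
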(event Custom|StartElec
  (Variables|Default|SetisElecCut false))

(event Custom|ElecCut
  (Variables|Default|SetisElecCut true))

(event EventBeginPlay
  (bind _returnvalue (Actor|GetActorOfClass "/Game/Blueprint/SpaceShip/BP_SpaceShipAsset.BP_SpaceShipAsset_C"))
  (Variables|Default|SetSpaceShip _returnvalue)
  (bind _returnvalue_2 (Actor|GetActorOfClass "/Game/Blueprint/SpaceShip/BP_BatterieSlot.BP_BatterieSlot_C"))
  (EventDispatchers|BindEventtoEDCutElec _returnvalue_2 (delegate Custom|ElecCut))
  (EventDispatchers|BindEventtoEDStartElec _returnvalue_2 (delegate Custom|StartElec)))

(event EventTick
  (params (DeltaSeconds :type Float%20%28single-precision%29))
  (bind _spaceship (Variables|Default|GetSpaceShip))
  (bind _waypoints (Variables|/Game/Blueprint/SpaceShip/BP_SpaceShipAsset.BP_SpaceShipAsset_C|GetWaypoints _spaceship))
  (Variables|Default|SetDelta%20Seconds DeltaSeconds)
  (Utilities|FlowControl|Sequence
    (:then_0
      (if (and (< (Math|Vector|Distance(Vector) (Transformation|GetWorldLocation (Variables|Default|GetMinster)) (Transformation|GetWorldLocation (Variables|/Game/Blueprint/SpaceShip/BP_SpaceShipAsset.BP_SpaceShipAsset_C|Getparent (Variables|Default|GetSpaceShip)))) 4e+02) (not (Variables|Default|GetisElecCut)))
        (if (not (Variables|Default|GethaveAttacked))
          (Default|LaunchOxygenLeak (Variables|Default|GetSpaceShip) 2.0 1e+01)
          (Variables|Default|SethaveAttacked true)
          (Development|PrintString "Hello"))))
    (:then_1
      (if (not (Variables|Default|GetisMoving))
        (Variables|Default|SetisMoving true)
        (Transformation|SetActorLocation (Transformation|GetWorldLocation (Utilities|Array|Get(acopy) _waypoints (Math|Random|RandomIntegerinRange 0 (- (Utilities|Array|Length _waypoints) 1)))) false false)
        (Utilities|FlowControl|Delay (Variables|Default|GetTpTime))
        (Variables|Default|SetisMoving false)))))

(fn ConstructionScript)