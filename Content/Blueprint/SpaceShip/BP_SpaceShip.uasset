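; Spaceship Blueprint that tracks an oxygen supply and simulates leaks.
; BeginPlay fills oxygen to its maximum and scales the oxygen bar component along X to match.
; LaunchOxygenLeak loops on a delay while the leak flag is set, each pass removing a percentage of the current oxygen, so the loss is exponential.
; The leak loop never refreshes the bar, and the joystick input event is an empty stub.
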(event Custom|LaunchOxygenLeak
  (params (Percentage :type Float%20%28double-precision%29))
  (if (Variables|Default|GetisOxygenLeaking?) :!label _label
    (CallFunction|OxygenLeak Percentage)
    (Utilities|FlowControl|Delay (Variables|Default|GetLeakTime))
    (goto _label)))

(event EventBeginPlay
  (bind _output_get (Variables|Default|SetOxygen (Variables|Default|GetOxygenMax)))
  (CallFunction|SetOxygenBarVisual (* _output_get 5.0)))

(event EventJoystickInput
  (params (JoystickInput :type Vector :default "0, 0, 0")))

(fn ConstructionScript)

(fn OxygenLeak
  (params (Percentage :type Float%20%28double-precision%29))
  (Variables|Default|SetOxygen (|(a-(a*(b/100))) (Variables|Default|GetOxygen) Percentage)))

(fn SetOxygenBarVisual
  (params (ScaleX :type Float%20%28double-precision%29))
  (bind _oxygenebar (Variables|Default|GetOxygeneBar))
  (bind _relativescale3d (Variables|/Script/Engine.SceneComponent|GetRelativeScale3D _oxygenebar))
  (Transformation|SetRelativeScale3D _oxygenebar (Math|Vector|MakeVector ScaleX (.y _relativescale3d) (.z _relativescale3d))))